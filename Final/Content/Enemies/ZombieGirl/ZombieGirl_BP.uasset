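; ZombieGirl_BP is a zombie enemy with physically animated hit-body motion, a melee attack and ragdoll death.
; Shortly after BeginPlay, a helper enables simulation and applies physical animation strengths below the spine and both upper legs, blending physics with animation.
; The HealthComponent death event clears the anim class, ragdolls the mesh with relaxed physical animation, then destroys the actor after a delay.
; An Attack event plays the melee montage.
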(event `self.ReceiveBeginPlay`
  (bind _physicalanimation (`self.PhysicalAnimation`))
  (bind _mesh (`self.Mesh`))
  (`|ExecutionSequence`
    (:`then_0`
      ;[1 1 1] Add Physical Animation
      (`KismetSystemLibrary.Delay` 0.075)
      (`PhysicalAnimationComponent.SetSkeletalMeshComponent` (`self.PhysicalAnimation`) (`self.Mesh`))
      (`|ExecutionSequence`
        (:`then_0`
          (`self.AddPhysicalAnimation` _physicalanimation _mesh "Spine1"))
        (:`then_1`
          (`self.AddPhysicalAnimation` _physicalanimation _mesh "RightUpLeg"))
        (:`then_2`
          (`self.AddPhysicalAnimation` _physicalanimation _mesh "LeftUpLeg"))))
    (:`then_1`
      ;[1 1 1] On Death
      (`/Game/_Source/Components/HealthComponent.BindOnDeath` (`self.HealthComponent`) (delegate `Death`)))))

(event `Death`
  (bind _mesh (`self.Mesh`))
  ;[1 1 1] On Death
  (`KismetSystemLibrary.PrintString` "ZOMBIE GIRL IS DEAD")
  (clear `/Game/_Source/Components/HealthComponent.OnDeathDispatcher` (`self.HealthComponent`))
  (`SkeletalMeshComponent.SetAnimInstanceClass` _mesh null)
  (`PrimitiveComponent.SetSimulatePhysics` _mesh true)
  (`PhysicalAnimationComponent.ApplyPhysicalAnimationSettingsBelow` (`self.PhysicalAnimation`) "None" (make `PhysicalAnimationData` true) true)
  (`KismetSystemLibrary.Delay` 5.0)
  (`self.K2_DestroyActor`))

(event `/Game/Enemies/IEnemy.Attack`
  (`|PlayMontage` (`self.Mesh`) "/Game/Enemies/ZombieGirl/Animation/AttackMelee.AttackMelee"))

(fn `AddPhysicalAnimation`
  (params (PhysicalAnimationComponent :type "PhysicalAnimationComponent Object Reference") (SkeletalMesh :type "SkeletalMeshComponent Object Reference") (BoneName :type Name))
  (`PhysicalAnimationComponent.ApplyPhysicalAnimationSettingsBelow` PhysicalAnimationComponent BoneName (make `PhysicalAnimationData` false 250.0 25.0 250.0 25.0) true)
  (`SkeletalMeshComponent.SetAllBodiesBelowSimulatePhysics` SkeletalMesh BoneName true true))

(fn `UserConstructionScript`)